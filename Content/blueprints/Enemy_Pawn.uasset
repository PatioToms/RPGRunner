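; Enemy pawn Blueprint that shows a highlight when its collider is clicked.
; The construction script gives the highlight component a dynamic material instance tinted by HighlightColor.
; On BeginPlay it caches the Touch_Gamemode reference, printing an error if the cast fails, though these graphs do not use that reference further.
; The click event only prints a debug message and makes the highlight visible, with no logic here to hide it again.
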(event OnClicked(EnemyCollider)
  (params (TouchedComponent :type Primitive%20Component%20Object%20Reference) (ButtonPressed :type Key%20Structure :default "AnyKey"))
  (Development|PrintString "Received Input")
  (Rendering|SetVisibility (Variables|Default|GetEnemyHighlight) true false))

(event EventBeginPlay
  (bind _astouch_gamemode (Utilities|Casting|CastToTouch_Gamemode (Game|GetGameMode))
    (:then
      (Variables|Default|SetGameModeReference _astouch_gamemode))
    (:CastFailed
      (Development|PrintString "ERROR: Enemy cast to game mode failed" true true "(R=1.000000,G=0.000000,B=0.039068,A=1.000000)" 4.0))))

(fn ConstructionScript
  (bind _returnvalue (Rendering|Material|CreateDynamicMaterialInstance (Variables|Default|GetEnemyHighlight) 0 "/Game/textures/mat_highlight.mat_highlight" :!class /Script/Engine.PrimitiveComponent))
  (Rendering|Material|SetVectorParameterValue _returnvalue "Tint" (Variables|Default|GetHighlightColor) :!class /Script/Engine.MaterialInstanceDynamic))