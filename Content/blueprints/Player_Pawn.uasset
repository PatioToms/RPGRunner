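; Player character pawn for a touch-driven 2D game, selected by clicking its collider and able to attack and take damage.
; Construction looks up CharacterID in a data table to set stats, flipbooks and tinted dynamic highlight materials.
; SelectCharacter allows one selection at a time through Touch_Gamemode and toggles the highlight sprites.
; Attacks deselect the pawn and step through timed sprite states; damage flashes the materials, reduces health and deselects, without triggering death.
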(event OnClicked(CharacterCollider)
  (params (TouchedComponent :type Primitive%20Component%20Object%20Reference) (ButtonPressed :type Key%20Structure :default "AnyKey"))
  (Development|PrintString "Received Player Input")
  (CallFunction|SelectCharacter (not (Variables|Default|GetIsSelected))))

(event Custom|ReceiveDamage
  (params (IncomingDamage :type Float%20%28single-precision%29))
  (Utilities|FlowControl|Sequence
    (:then_0
      ;[1 1 1] Cosmetic Effect when receiving damage
      (bind _materialalpha (Timeline|DamageEffectTimeline PlayFromStart)
        (:Update
          (Rendering|Material|SetScalarParameterValue (Variables|Default|GetCharacterSpriteMaterial) "AlphaBlend" _materialalpha :!class /Script/Engine.MaterialInstanceDynamic))))
    (:then_1
      (Variables|Default|SetCurrentHealth (- (Variables|Default|GetCurrentHealth) IncomingDamage))
      (CallFunction|SelectCharacter false))))

(event Custom|AttackEnemy
  (bind _output_get (Variables|Default|SetIsSelectable false))
  (Utilities|FlowControl|Sequence
    (:then_0
      (CallFunction|SelectCharacter _output_get))
    (:then_1
      (CallFunction|ChangeSpriteState "NewEnumerator1")
      (Utilities|FlowControl|Delay (Variables|Default|GetAttackDuration))
      (CallFunction|ChangeSpriteState "NewEnumerator2")
      (Utilities|FlowControl|Delay (Variables|Default|GetDefaultReloadSpeed))
      (if (not (Variables|Default|GetIsDead))
        (CallFunction|ChangeSpriteState "NewEnumerator0")
        (Variables|Default|SetIsSelectable true)))))

(event EventBeginPlay
  (bind _astouch_gamemode (Utilities|Casting|CastToTouch_Gamemode (Game|GetGameMode))
    (:then
      (Variables|Default|SetGameModeReference _astouch_gamemode))
    (:CastFailed
      (Development|PrintString "ERROR: Cast to Game Mode Failed (from character pawn)" true true "(R=1.000000,G=0.000000,B=0.037282,A=1.000000)" 4.0))))

(fn ConstructionScript
  ;[1 1 1] Character Setup (based on the CharacterID variable
  (bind _returnvalue (Utilities|GetDataTableRow "/Game/data/player_datatable.player_datatable" (Utilities|String|StringToName (Utilities|String|ToString(Integer) (Variables|Default|GetCharacterID))))
    (:then
      (Utilities|FlowControl|Sequence
        (:then_0
          ;;[1 1 1] We set up the character simple values like health, attack and reload speed
          (bind _output_get (Variables|Default|SetDefaultHealth (.Health (Utilities|Struct|Breakplayer_struct _returnvalue))))
          (Variables|Default|SetCurrentHealth _output_get)
          (Variables|Default|SetDefaultAttack (.Attack (Utilities|Struct|Breakplayer_struct _returnvalue)))
          (Variables|Default|SetDefaultReloadSpeed (.ReloadSpeed (Utilities|Struct|Breakplayer_struct _returnvalue)))
          (Variables|Default|SetAttackDuration (.AttackDuration (Utilities|Struct|Breakplayer_struct _returnvalue)))
          (Variables|Default|SetDeathDuration (.DeathDuration (Utilities|Struct|Breakplayer_struct _returnvalue))))
        (:then_1
          ;;[1 1 1] We set up the character sprites
          (Utilities|FlowControl|Sequence
            (:then_0
              (bind _output_get_2 (Variables|Default|SetCharacterIdle (.IdleSprite (Utilities|Struct|Breakplayer_struct _returnvalue))))
              (Sprite|SetFlipbook (Variables|Default|GetCharacterSprite) _output_get_2)
              (Sprite|SetFlipbook (Variables|Default|GetCharacterHighlight) _output_get_2))
            (:then_1
              (Variables|Default|SetCharacterAttack (.AttackSprite (Utilities|Struct|Breakplayer_struct _returnvalue))))
            (:then_2
              (Variables|Default|SetCharacterReload (.ReloadSprite (Utilities|Struct|Breakplayer_struct _returnvalue))))
            (:then_3
              (Variables|Default|SetCharacterDying (.DyingSprite (Utilities|Struct|Breakplayer_struct _returnvalue))))
            (:then_4
              (Variables|Default|SetCharacterDead (.DeadSprite (Utilities|Struct|Breakplayer_struct _returnvalue))))
            (:then_5
              (bind _output_get_3 (Variables|Default|SetWeaponIdle (.WeaponIdleSprite (Utilities|Struct|Breakplayer_struct _returnvalue))))
              (Sprite|SetFlipbook (Variables|Default|GetWeaponSprite) _output_get_3)
              (Sprite|SetFlipbook (Variables|Default|GetWeaponHightlight) _output_get_3))
            (:then_6
              (Variables|Default|SetWeaponReload (.WeaponReloadSprite (Utilities|Struct|Breakplayer_struct _returnvalue))))
            (:then_7
              (Variables|Default|SetWeaponAttack (.WeaponAttackSprite (Utilities|Struct|Breakplayer_struct _returnvalue))))
            (:then_8
              (Variables|Default|SetWeaponDying (.WeaponDyingSprite (Utilities|Struct|Breakplayer_struct _returnvalue))))
            (:then_9
              (Variables|Default|SetWeaponDead (.WeaponDeadSprite (Utilities|Struct|Breakplayer_struct _returnvalue))))))
        (:then_2
          ;;[1 1 1] We set up the character's aesthetic aspects
          (Utilities|FlowControl|Sequence
            (:then_0
              (Variables|Default|SetCharacter%20Name (.CharacterName (Utilities|Struct|Breakplayer_struct _returnvalue))))
            (:then_1
              (bind _output_get_4 (Variables|Default|SetHighlightColor (.HighlightColor (Utilities|Struct|Breakplayer_struct _returnvalue))))
              (bind _returnvalue_2 (Rendering|Material|CreateDynamicMaterialInstance (Variables|Default|GetWeaponHightlight) 0 "/Game/textures/mat_highlight.mat_highlight" :!class /Script/Engine.PrimitiveComponent))
              (bind _output_get_5 (Variables|Default|SetWeaponHighlightMaterial _returnvalue_2))
              (Rendering|Material|SetVectorParameterValue _output_get_5 "Tint" _output_get_4 :!class /Script/Engine.MaterialInstanceDynamic)
              (bind _returnvalue_3 (Rendering|Material|CreateDynamicMaterialInstance (Variables|Default|GetWeaponSprite) 0 "/Game/textures/mat_sprites_main.mat_sprites_main" :!class /Script/Engine.PrimitiveComponent))
              (Variables|Default|SetWeaponSpriteMaterial _returnvalue_3))
            (:then_2
              (bind _returnvalue_4 (Rendering|Material|CreateDynamicMaterialInstance (Variables|Default|GetCharacterHighlight) 0 "/Game/textures/mat_highlight.mat_highlight" :!class /Script/Engine.PrimitiveComponent))
              (bind _output_get_6 (Variables|Default|SetCharacterHighlightMaterial _returnvalue_4))
              (Rendering|Material|SetVectorParameterValue _output_get_6 "Tint" _output_get_4 :!class /Script/Engine.MaterialInstanceDynamic)
              (bind _returnvalue_5 (Rendering|Material|CreateDynamicMaterialInstance (Variables|Default|GetCharacterSprite) 0 "/Game/textures/mat_sprites_main.mat_sprites_main" :!class /Script/Engine.PrimitiveComponent))
              (Variables|Default|SetCharacterSpriteMaterial _returnvalue_5))))))
    (:RowNotFound
      (Development|PrintString "ERROR: Character ID not valid" true true "(R=1.000000,G=0.000000,B=0.066323,A=1.000000)" 4.0))))

(fn SelectCharacter
  (params (New%20State :type Boolean))
  (bind _gamemodereference (Variables|Default|GetGameModeReference))
  (if New%20State
    (if (and (Variables|Default|GetIsSelectable) (not (Variables|/Game/blueprints/Touch_Gamemode.Touch_Gamemode_C|GetIsCharacterSelected (Variables|Default|GetGameModeReference))))
      (Utilities|FlowControl|Sequence :!label _label
        (:then_0
          (bind _output_get (Variables|/Game/blueprints/Touch_Gamemode.Touch_Gamemode_C|SetIsCharacterSelected _gamemodereference New%20State))
          (if _output_get
            (Variables|/Game/blueprints/Touch_Gamemode.Touch_Gamemode_C|SetSelectedCharacter _gamemodereference self)
            (Development|PrintString (Utilities|String|Append (Variables|Default|GetCharacter%20Name) " selected"))
            (else
              (Variables|/Game/blueprints/Touch_Gamemode.Touch_Gamemode_C|SetSelectedCharacter _gamemodereference 0)
              (Development|PrintString (Utilities|String|Append (Variables|Default|GetCharacter%20Name) " unselected")))))
        (:then_1
          (Rendering|SetVisibility (Variables|Default|GetCharacterHighlight) New%20State false))
        (:then_2
          (Variables|Default|SetIsSelected New%20State)))
      (else
        (Development|PrintString "ERROR: Pawn does not meet criteria to be selected" true true "(R=1.000000,G=0.000000,B=0.000000,A=1.000000)")))
    (elif (== (Variables|/Game/blueprints/Touch_Gamemode.Touch_Gamemode_C|GetSelectedCharacter (Variables|Default|GetGameModeReference)) self)
      (goto _label)
      (else
        (Development|PrintString "Error: Pawn ID not valid" true true "(R=1.000000,G=0.000000,B=0.000000,A=1.000000)")))))

(fn ChangeSpriteState
  (params (NewState :type player_states%20Enum))
  (bind _characteridle (Variables|Default|GetCharacterIdle))
  (bind _weaponidle (Variables|Default|GetWeaponIdle))
  (bind _weaponreload (Variables|Default|GetWeaponReload))
  (bind _characterreload (Variables|Default|GetCharacterReload))
  (bind _weaponattack (Variables|Default|GetWeaponAttack))
  (bind _characterattack (Variables|Default|GetCharacterAttack))
  (bind _characterdying (Variables|Default|GetCharacterDying))
  (bind _characterdead (Variables|Default|GetCharacterDead))
  (bind _weapondead (Variables|Default|GetWeaponDead))
  (bind _weapondying (Variables|Default|GetWeaponDying))
  (switch Utilities|FlowControl|Switch|Switchonplayer_states NewState
    (:NewEnumerator0
      (Sprite|SetFlipbook (Variables|Default|GetCharacterSprite) _characteridle)
      (Sprite|SetFlipbook (Variables|Default|GetCharacterHighlight) _characteridle)
      (Sprite|SetFlipbook (Variables|Default|GetWeaponSprite) _weaponidle)
      (Sprite|SetFlipbook (Variables|Default|GetWeaponHightlight) _weaponidle))
    (:NewEnumerator1
      (Sprite|SetFlipbook (Variables|Default|GetCharacterSprite) _characterattack)
      (Sprite|SetFlipbook (Variables|Default|GetCharacterHighlight) _characterattack)
      (Sprite|SetFlipbook (Variables|Default|GetWeaponSprite) _weaponattack)
      (Sprite|SetFlipbook (Variables|Default|GetWeaponHightlight) _weaponattack))
    (:NewEnumerator2
      (Sprite|SetFlipbook (Variables|Default|GetCharacterSprite) _characterreload)
      (Sprite|SetFlipbook (Variables|Default|GetCharacterHighlight) _characterreload)
      (Sprite|SetFlipbook (Variables|Default|GetWeaponSprite) _weaponreload)
      (Sprite|SetFlipbook (Variables|Default|GetWeaponHightlight) _weaponreload))
    (:NewEnumerator3
      (Sprite|SetFlipbook (Variables|Default|GetCharacterSprite) _characterdying)
      (Sprite|SetFlipbook (Variables|Default|GetCharacterHighlight) _characterdying)
      (Sprite|SetFlipbook (Variables|Default|GetWeaponSprite) _weapondying)
      (Sprite|SetFlipbook (Variables|Default|GetWeaponHightlight) _weapondying))
    (:NewEnumerator4
      (Sprite|SetFlipbook (Variables|Default|GetCharacterSprite) _characterdead)
      (Sprite|SetFlipbook (Variables|Default|GetCharacterHighlight) _characterdead)
      (Sprite|SetFlipbook (Variables|Default|GetWeaponSprite) _weapondead)
      (Sprite|SetFlipbook (Variables|Default|GetWeaponHightlight) _weapondead))))