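; Base projectile actor with a flipbook sprite that damages Enemy actors, typed as Flamethrower, Shotgun or SMG.
; The construction script maps Type to a data table row that sets speed, penetration, size, sprite and optional explosion.
; It moves forward per tick, unscaled by delta time, and expires on a timer.
; Hits on living enemies spend penetration; at zero it destroys itself, first expanding its box for half-damage splash if explosive.
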(event EventBeginPlay
  (Utilities|FlowControl|Delay 15.0)
  (Actor|DestroyActor))

(event Collision|EventActorBeginOverlap
  (params (OtherActor :type Actor%20Object%20Reference))
  (bind _explosionsize (Variables|Default|GetExplosionSize))
  (bind _asenemy (Utilities|Casting|CastToEnemy OtherActor))
  (if (not (Variables|/Game/blueprints/Enemy.Enemy_C|GetIsDead _asenemy))
    (Default|ReceiveDamage _asenemy (Variables|Default|GetDamage))
    (bind _result (Math|Integer|DecrementInt (Variables|Default|GetPenetration))
      (:%20%20
        (if (== _result 0)
          (if (> (Variables|Default|GetExplosionSize) 0.0)
            (Variables|Default|SetSpeed 1.0)
            ;[1 1 1] Projectile Explosion
            (Utilities|FlowControl|Sequence
              (:then_0
                (Sprite|SetFlipbook (Variables|Default|GetProjectileSprite) (Variables|Default|GetExplosionSprite)))
              (:then_1
                (Components|Box|SetBoxExtent (Variables|Default|GetBox) (Math|Vector|MakeVector _explosionsize 1e+02 _explosionsize) true)
                (for _array_element (Collision|GetOverlappingActors (Variables|Default|GetBox) 0 :!class /Script/Engine.PrimitiveComponent)
                  (if (== _array_element "/Game/blueprints/Enemy.Enemy")
                    (bind _asenemy_2 (Utilities|Casting|CastToEnemy _array_element))
                    (Default|ReceiveDamage _asenemy_2 (/ (Variables|Default|GetDamage) 2.0))))
                (Utilities|FlowControl|Delay 0.7)
                (Actor|DestroyActor :!label _label)))
            (else
              (goto _label))))))))

(event EventTick
  (params (DeltaSeconds :type Float%20%28single-precision%29))
  (Transformation|AddActorLocalOffset (Math|Vector|MakeVector (Variables|Default|GetSpeed) 0.0 0.0) false false))

(fn ConstructionScript
  (switch Utilities|FlowControl|Switch|Switchonprojectile_enum (Variables|Default|GetType)
    (:NewEnumerator2
      (LocalVariables|SetProjectileIndex 0))
    (:NewEnumerator0
      (LocalVariables|SetProjectileIndex 1))
    (:NewEnumerator1
      (LocalVariables|SetProjectileIndex 2)))
  (bind _returnvalue (Utilities|GetDataTableRow "/Game/data/projectile_datatable.projectile_datatable" (Utilities|String|StringToName (Utilities|String|ToString(Integer) (LocalVariables|GetProjectileIndex))))
    (:then
      (Utilities|FlowControl|Sequence
        (:then_0
          (Variables|Default|SetSpeed (.Speed (Utilities|Struct|Breakprojectile_struct _returnvalue)))
          (Variables|Default|SetPenetration (.Penetration (Utilities|Struct|Breakprojectile_struct _returnvalue))))
        (:then_1
          (Components|Box|SetBoxExtent (Variables|Default|GetBox) (Math|Vector|MakeVector (.Size (Utilities|Struct|Breakprojectile_struct _returnvalue)) 1e+02 (.Size (Utilities|Struct|Breakprojectile_struct _returnvalue))) true)
          (Sprite|SetFlipbook (Variables|Default|GetProjectileSprite) (.Sprite (Utilities|Struct|Breakprojectile_struct _returnvalue))))
        (:then_2
          (if (.DoesItExplode (Utilities|Struct|Breakprojectile_struct _returnvalue))
            (Utilities|FlowControl|Sequence
              (:then_0
                (Variables|Default|SetExplosionSize (.ExplosionSize (Utilities|Struct|Breakprojectile_struct _returnvalue))))
              (:then_1
                (Variables|Default|SetExplosionSprite (.ExplosionSprite (Utilities|Struct|Breakprojectile_struct _returnvalue)))))))))))