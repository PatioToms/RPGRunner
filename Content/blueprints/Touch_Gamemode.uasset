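; Touch_Gamemode is a game mode that brokers attacks between player characters and enemies.
; On BeginPlay it caches all placed Player_Pawn actors in PlayerArray, and its SpawnDefaultPawnFor override returns no pawn.
; AttackEnemy sends the selected character's default attack damage and highlight color to the target enemy, then calls that character's own AttackEnemy.
; AttackPlayer forwards incoming damage to the target character.
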(event EventBeginPlay
  (CallFunction|CreatePlayerArray))

(fn ConstructionScript)

(fn SpawnDefaultPawnfor
  (params (NewPlayer :type Controller%20Object%20Reference) (StartSpot :type Actor%20Object%20Reference))
  (return 0))

(fn AttackEnemy
  (params (TargetEnemy :type Enemy%20Object%20Reference))
  (bind _selectedcharacter (Variables|Default|GetSelectedCharacter))
  (Default|ReceiveDamage TargetEnemy (Variables|/Game/blueprints/Player_Pawn.Player_Pawn_C|GetDefaultAttack _selectedcharacter) (Variables|/Game/blueprints/Player_Pawn.Player_Pawn_C|GetHighlightColor _selectedcharacter))
  (Default|AttackEnemy _selectedcharacter))

(fn AttackPlayer
  (params (Target%20Character :type Player%20Pawn%20Object%20Reference) (Incoming%20Damage :type Float%20%28single-precision%29))
  (Default|ReceiveDamage Target%20Character Incoming%20Damage))

(fn CreatePlayerArray
  (bind _outactors (Actor|GetAllActorsOfClass "/Game/blueprints/Player_Pawn.Player_Pawn_C"))
  (Variables|Default|SetPlayerArray _outactors))