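; Clickable Paper2D enemy actor that the selected character can attack through Touch_Gamemode.
; InitiateEnemy loads stats, flipbooks, scale and tint from Enemy_datatable by EnemyID, and ChangeEnemyState swaps sprite and highlight flipbooks together.
; ReceiveDamage blocks selection, shows a player-colored highlight and runs a material-blend timeline, then restores selection or plays death and destroys the actor.
; LocateTarget only stores a target and an offset attack position; no movement happens here.
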(event OnClicked(EnemyCollider)
  (params (TouchedComponent :type Primitive%20Component%20Object%20Reference) (ButtonPressed :type Key%20Structure :default "AnyKey"))
  (Development|PrintString "Enemy received Input")
  (if (and (Variables|/Game/blueprints/Touch_Gamemode.Touch_Gamemode_C|GetIsCharacterSelected (Variables|Default|GetGameModeReference)) (Variables|Default|GetIsSelectable))
    (Default|AttackEnemy (Variables|Default|GetGameModeReference) self)
    (else
      (Development|PrintString "Enemy selection not valid" true true "(R=0.909452,G=0.000000,B=1.000000,A=1.000000)"))))

(event Custom|ReceiveDamage
  (params (PlayerDamage :type Float%20%28single-precision%29) (PlayerColor :type Linear%20Color%20Structure))
  ;[1 1 1] Function for taking damage
  (Variables|Default|SetIsSelectable false)
  (Rendering|Material|SetVectorParameterValue (Variables|Default|GetEnemyHighlightMaterial) "Tint" PlayerColor :!class /Script/Engine.MaterialInstanceDynamic)
  (Rendering|SetVisibility (Variables|Default|GetEnemyHighlight) true false)
  (Variables|Default|SetHealth (- (Variables|Default|GetHealth) PlayerDamage))
  (bind _materialalpha (Timeline|DamageTimeline PlayFromStart)
    (:Update
      (Rendering|Material|SetScalarParameterValue (Variables|Default|GetEnemySpriteMaterial) "AlphaBlend" _materialalpha :!class /Script/Engine.MaterialInstanceDynamic))
    (:Finished
      (if (<= (Variables|Default|GetHealth) 0.0)
        ;[1 1 1] Enemy Death
        (Development|PrintString "I AM DED" true true "(R=0.000000,G=1.000000,B=0.144330,A=1.000000)" 5.0)
        (CallFunction|ChangeEnemyState "NewEnumerator3")
        (Utilities|FlowControl|Delay (Variables|Default|GetDeathTime))
        (Actor|DestroyActor)
        (else
          (Development|PrintString (Utilities|String|Append (Utilities|GetObjectName self) " Health: " (Utilities|String|ToString(Float) (Variables|Default|GetHealth))))
          (Rendering|SetVisibility (Variables|Default|GetEnemyHighlight) false false)
          (Variables|Default|SetIsSelectable true))))))

(event Custom|RetryGettingGamemode
  ;[1 1 1] Getting Game Mode
  (bind _astouch_gamemode (Utilities|Casting|CastToTouch_Gamemode (Game|GetGameMode))
    (:then
      (Variables|Default|SetGameModeReference _astouch_gamemode))
    (:CastFailed
      (Development|PrintString "ERROR: Enemy cast to game mode failed" true true "(R=1.000000,G=0.000000,B=0.039068,A=1.000000)" 4.0)
      (CallFunction|RetryGettingGamemode))))

(event EventBeginPlay
  (Utilities|FlowControl|Sequence
    (:then_0
      ;[1 1 1] Getting Game Mode
      (bind _astouch_gamemode (Utilities|Casting|CastToTouch_Gamemode (Game|GetGameMode))
        (:then
          (Variables|Default|SetGameModeReference _astouch_gamemode))
        (:CastFailed
          (Development|PrintString "ERROR: Enemy cast to game mode failed" true true "(R=1.000000,G=0.000000,B=0.039068,A=1.000000)" 4.0)
          (CallFunction|RetryGettingGamemode))))))

(fn ConstructionScript
  (Utilities|FlowControl|Sequence
    (:then_0
      (bind _returnvalue (Rendering|Material|CreateDynamicMaterialInstance (Variables|Default|GetEnemyHighlight) 0 "/Game/textures/mat_highlight.mat_highlight" :!class /Script/Engine.PrimitiveComponent))
      (Variables|Default|SetEnemyHighlightMaterial _returnvalue))
    (:then_1
      (bind _returnvalue_2 (Rendering|Material|CreateDynamicMaterialInstance (Variables|Default|GetEnemySprite) 0 "/Game/textures/mat_sprites_main.mat_sprites_main" :!class /Script/Engine.PrimitiveComponent))
      (Variables|Default|SetEnemySpriteMaterial _returnvalue_2))))

(fn InitiateEnemy
  (bind _returnvalue (Transformation|GetActorLocation))
  (bind (_x _y _z) (Math|Vector|BreakVector _returnvalue))
  (bind _returnvalue_2 (Utilities|GetDataTableRow "/Game/data/enemy_datatable.enemy_datatable" (Utilities|String|StringToName (Utilities|String|ToString(Integer) (Variables|Default|GetEnemy_ID))))
    (:then
      (Utilities|FlowControl|Sequence
        (:then_0
          ;[1 1 1] Setting up variables and scale
          (Transformation|SetWorldScale3D (Variables|Default|GetEnemySprite) (Math|Conversions|ToVector(Float) (.SpriteScale (Utilities|Struct|Breakenemy_struct _returnvalue_2))))
          (Variables|Default|SetDeathTime (.DeathDuration (Utilities|Struct|Breakenemy_struct _returnvalue_2)))
          (Variables|Default|SetAttackTime (.AttackDuration (Utilities|Struct|Breakenemy_struct _returnvalue_2)))
          (Variables|Default|SetWaveWeight (.WaveWeight (Utilities|Struct|Breakenemy_struct _returnvalue_2)))
          (Variables|Default|SetHealth (.Health (Utilities|Struct|Breakenemy_struct _returnvalue_2)))
          (Variables|Default|SetSpeed (.Speed (Utilities|Struct|Breakenemy_struct _returnvalue_2)))
          (Variables|Default|SetAttack (.Attack (Utilities|Struct|Breakenemy_struct _returnvalue_2))))
        (:then_1
          ;[1 1 1] Setting up the enemy sprite
          (Utilities|FlowControl|Sequence
            (:then_0
              (Variables|Default|SetMoveSprite (.MoveSprite (Utilities|Struct|Breakenemy_struct _returnvalue_2))))
            (:then_1
              (Variables|Default|SetIdleSprite (.IdleSprite (Utilities|Struct|Breakenemy_struct _returnvalue_2))))
            (:then_2
              (Variables|Default|SetAttackSprite (.AttackSprite (Utilities|Struct|Breakenemy_struct _returnvalue_2))))
            (:then_3
              (Variables|Default|SetDeathSprite (.DeathSprite (Utilities|Struct|Breakenemy_struct _returnvalue_2))))
            (:then_4
              (Rendering|Material|SetVectorParameterValue (Variables|Default|GetEnemySpriteMaterial) "Tint" (.SpriteTint (Utilities|Struct|Breakenemy_struct _returnvalue_2)) :!class /Script/Engine.MaterialInstanceDynamic))))
        (:then_2
          ;[1 1 1] Setting up enemy location
          (Transformation|SetActorLocation (Math|Vector|MakeVector _x (Variables|Default|GetYLocation) _z) false true))))))

(fn ChangeEnemyState
  (params (New%20State :type enemy_states%20Enum))
  (bind _deathsprite (Variables|Default|GetDeathSprite))
  (bind _attacksprite (Variables|Default|GetAttackSprite))
  (bind _idlesprite (Variables|Default|GetIdleSprite))
  (bind _movesprite (Variables|Default|GetMoveSprite))
  (switch Utilities|FlowControl|Switch|Switchonenemy_states New%20State
    (:NewEnumerator0
      (Sprite|SetFlipbook (Variables|Default|GetEnemySprite) _movesprite)
      (Sprite|SetFlipbook (Variables|Default|GetEnemyHighlight) _movesprite))
    (:NewEnumerator1
      (Sprite|SetFlipbook (Variables|Default|GetEnemySprite) _idlesprite)
      (Sprite|SetFlipbook (Variables|Default|GetEnemyHighlight) _idlesprite))
    (:NewEnumerator2
      (Sprite|SetFlipbook (Variables|Default|GetEnemySprite) _attacksprite)
      (Sprite|SetFlipbook (Variables|Default|GetEnemyHighlight) _attacksprite))
    (:NewEnumerator3
      (Sprite|SetFlipbook (Variables|Default|GetEnemySprite) _deathsprite)
      (Sprite|SetFlipbook (Variables|Default|GetEnemyHighlight) _deathsprite))))

(fn LocateTarget
  (params (NewTarget :type Player%20Pawn%20Object%20Reference))
  (bind _returnvalue (Transformation|GetActorLocation NewTarget))
  (bind (_x _y _z) (Math|Vector|BreakVector _returnvalue))
  (Variables|Default|SetTargetReference NewTarget)
  (Variables|Default|SetTargetLocation (Math|Vector|MakeVector (+ _x (Variables|Default|GetAttackDistance)) (Variables|Default|GetYLocation) _z)))